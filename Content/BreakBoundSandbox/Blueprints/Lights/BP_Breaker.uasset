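; BP_Breaker is an interactable circuit breaker that trips when its linked lights draw too much power.
; On BeginPlay it binds to each light's OnFireBreaker dispatcher and runs CheckBreaker, which sums lit lights' power usage after a short retriggerable delay.
; Exceeding MaxPower turns off all linked lights, deactivates the breaker and turns its mesh red.
; Interacting only re-arms a tripped breaker and turns it green, without relighting the lights.
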(event Custom|CheckBreaker
  (if (Variables|Default|GetbIsActive)
    (Utilities|FlowControl|RetriggerableDelay 0.2)
    (Variables|Default|SetCurrentPower 0.0)
    (for _array_element (Variables|Default|GetLights)
      (if (Variables|/Game/BreakBoundSandbox/Blueprints/Lights/BP_Lights_Base.BP_Lights_Base_C|GetbIsLightOn _array_element)
        (bind _output_get (Variables|Default|SetCurrentPower (+ (Variables|Default|GetCurrentPower) (Variables|/Game/BreakBoundSandbox/Blueprints/Lights/BP_Lights_Base.BP_Lights_Base_C|GetPowerUssage _array_element))))
        (Development|PrintString (Utilities|String|ToString(Float) _output_get))))
    (if (> (Variables|Default|GetCurrentPower) (Variables|Default|GetMaxPower))
      (for _array_element_2 (Variables|Default|GetLights)
        (Default|TurnOffLights _array_element_2)
        (CallFunction|RefreshBreaker false)
        (Variables|Default|SetbIsActive false)))))

(event EventBeginPlay
  (Utilities|FlowControl|Sequence
    (:then_0
      (for _array_element (Variables|Default|GetLights)
        (Utilities|IsValid _array_element
          (:Is%20Valid
            (EventDispatchers|AssignOnFireBreaker _array_element (EventDispatchers|CreateEvent :!event Custom|CheckBreaker))))))
    (:then_1
      (CallFunction|CheckBreaker))))

(event EventOnInteract
  (CallFunction|SwitchBreaker))

(fn ConstructionScript)

(fn RefreshBreaker
  (params (Enabled :type Boolean))
  (Rendering|Material|CreateDynamicMaterialInstance (Variables|Default|GetBreakerMesh) 0 (select Enabled "/Game/BreakBoundSandbox/Materials/Interaction/M_Green.M_Green" "/Game/BreakBoundSandbox/Materials/Interaction/M_Red.M_Red") "None" :!class /Script/Engine.PrimitiveComponent))

(fn SwitchBreaker
  (if (not (Variables|Default|GetbIsActive))
    (Variables|Default|SetbIsActive true)
    (CallFunction|RefreshBreaker true)))

(fn GetCamera
  (return 0))

(fn GetItemData
  (return ""))