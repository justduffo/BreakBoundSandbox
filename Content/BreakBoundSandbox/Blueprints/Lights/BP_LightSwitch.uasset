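; BP_LightSwitch is an interactable wall switch that controls an assigned list of lights.
; On interact it plays a switch sound at its location and sends CycleLightsMessage to every light in LightsToInteract.
; The construction script uses IsLightOn to send turn-on or turn-off messages to those lights; interacting does not update that flag.
; GetCamera and GetItemData are empty stubs.
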(event EventBeginPlay)

(event Collision|EventActorBeginOverlap
  (params (OtherActor :type Actor%20Object%20Reference)))

(event EventTick
  (params (DeltaSeconds :type Float%20%28single-precision%29)))

(event EventOnInteract
  (Audio|PlaySoundatLocation "/Game/BreakBoundSandbox/Sounds/Cues/wav_Lightswitch_Cue.wav_Lightswitch_Cue" (Transformation|GetActorLocation) "0, 0, 0" 1.0 1.0 0.0 0 0 0 0)
  (for _array_element (Variables|Default|GetLightsToInteract)
    (Class|BPILights|CycleLights(Message) _array_element)))

(fn ConstructionScript
  (if (Variables|Default|GetbIsLightOn)
    (for _array_element (Variables|Default|GetLightsToInteract)
      (Class|BPILights|TurnonLIghts(Message) _array_element))
    (else
      (for _array_element_2 (Variables|Default|GetLightsToInteract)
        (Class|BPILights|TurnOffLights(Message) _array_element_2)))))

(fn GetCamera
  (return 0))

(fn GetItemData
  (return ""))