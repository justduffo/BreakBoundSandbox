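; Base light actor for BreakBoundSandbox, a spotlight fixture with a bulb that switches on and off subject to a linked breaker.
; The construction script applies the configurable mesh, transform, cone, color, radius and initial intensity.
; CycleLights toggles the light only if CheckBreaker, which also calls CallOnFireBreaker, finds the BP_Breaker active.
; The on and off events set spotlight intensity, swap the bulb material through dynamic instances and update IsLightOn.
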(event EventCycleLights
  (bind _isactive (CallFunction|CheckBreaker))
  (if _isactive
    (if (Variables|Default|GetbIsLightOn)
      (CallFunction|TurnOffLights)
      (else
        (CallFunction|TurnonLIghts)))))

(event EventTurnOffLights
  (Rendering|Components|Light|SetIntensity (Variables|Default|GetSpotLight) 0.0)
  (Rendering|Material|CreateDynamicMaterialInstance (Variables|Default|GetBulb) 0 "/Game/BreakBoundSandbox/Materials/Lights/M_Bulb.M_Bulb" "None" :!class /Script/Engine.PrimitiveComponent)
  (Variables|Default|SetbIsLightOn false))

(event EventTurnonLIghts
  (Rendering|Components|Light|SetIntensity (Variables|Default|GetSpotLight) (Variables|Default|GetIntensity))
  (Rendering|Material|CreateDynamicMaterialInstance (Variables|Default|GetBulb) 0 "/Game/BreakBoundSandbox/Materials/Lights/M_BulbOn.M_BulbOn" "None" :!class /Script/Engine.PrimitiveComponent)
  (Variables|Default|SetbIsLightOn true))

(fn ConstructionScript
  (bind _spotlight (Variables|Default|GetSpotLight))
  (Utilities|FlowControl|Sequence
    (:then_0
      (Components|StaticMesh|SetStaticMesh (Variables|Default|GetLightBase) (Variables|MeshSettings|GetLightMesh))
      (Transformation|SetRelativeLocation (Variables|Default|GetLightBase) (Variables|MeshSettings|GetLightBaseLocation) false false)
      (Transformation|SetRelativeScale3D (Variables|Default|GetLightBase) (Math|Conversions|ToVector(Float) (Variables|MeshSettings|GetLightMeshScale)))
      (Transformation|SetRelativeRotation (Variables|Default|GetLightBase) (Variables|MeshSettings|GetLightBaseRotation) false false))
    (:then_1
      (Rendering|Lighting|SetAttenuationRadius _spotlight (Variables|LightSettings|GetAttenuationRadius))
      (Rendering|Lighting|SetInnerConeAngle _spotlight (Variables|LightSettings|GetInnerConeAngle))
      (Rendering|Lighting|SetOuterConeAngle _spotlight (Variables|LightSettings|GetOuterConeAngle))
      (Rendering|Components|Light|SetLightColor _spotlight (Variables|LightSettings|GetLightColor) true))
    (:then_2
      (Rendering|Components|Light|SetIntensity (Variables|Default|GetSpotLight) (Math|Float|SelectFloat (Variables|Default|GetIntensity) 0.0 (Variables|Default|GetbIsLightOn))))))

(fn CheckBreaker
  (bind _asbp_breaker (Utilities|Casting|CastToBP_Breaker (Variables|Default|GetBreaker)))
  (Default|CallOnFireBreaker)
  (if (Variables|/Game/BreakBoundSandbox/Blueprints/Lights/BP_Breaker.BP_Breaker_C|GetbIsActive _asbp_breaker)
    (return true)
    (else
      (return false))))