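; BP_InteractionMaster is an interactable actor with placeholder responses to interaction and focus.
; OnInteract only prints a debug message, and GetItemData returns the item name.
; Focused turns the static mesh green, then restores the grey material after a short retriggerable delay, so repeated focus calls keep the highlight active without a separate unfocus event.
; GetCamera is an empty stub.
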(event EventBeginPlay)

(event Collision|EventActorBeginOverlap
  (params (OtherActor :type Actor%20Object%20Reference)))

(event EventTick
  (params (DeltaSeconds :type Float%20%28single-precision%29)))

(event EventOnInteract
  (Development|PrintString "Interacting"))

(event EventFocused
  (Rendering|Material|SetMaterial (Variables|Default|GetStaticMesh) 0 "/Game/BreakBoundSandbox/Materials/Interaction/M_Green.M_Green")
  (Utilities|FlowControl|RetriggerableDelay 0.2)
  (Rendering|Material|SetMaterial (Variables|Default|GetStaticMesh) 0 "/Engine/EditorMeshes/ColorCalibrator/M_GreyBall.M_GreyBall"))

(fn ConstructionScript)

(fn GetCamera
  (return 0))

(fn GetItemData
  (return (Variables|Default|GetItemName)))