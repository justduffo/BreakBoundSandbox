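; BP_Keys is an interactable key pickup that gives the player a key ID, located among the door actors.
; On interact, it gets the interaction component, shows a popup with its action text and adds its KeyID to that component's Keys.
; It then plays a 2D key jingle sound and destroys itself.
; GetCamera and GetItemData are stubs that return nothing useful.
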(event EventBeginPlay)

(event Collision|EventActorBeginOverlap
  (params (OtherActor :type Actor%20Object%20Reference)))

(event EventTick
  (params (DeltaSeconds :type Float%20%28single-precision%29)))

(event EventOnInteract
  (bind _interactioncomponent (CallFunction|GetInteractionComponent))
  (Default|DisplayPopup _interactioncomponent (Variables|Default|GetActionText))
  (Utilities|Array|Add (Variables|/Game/BreakBoundSandbox/Blueprints/Components/BPC_Interaction.BPC_Interaction_C|GetKeys _interactioncomponent) (Variables|Default|GetKeyID))
  (Audio|PlaySound2D "/Game/BreakBoundSandbox/Sounds/Cues/wav_Key_Jiggle_Cue.wav_Key_Jiggle_Cue" 1.0 1.0 0.0 0 0)
  (Actor|DestroyActor))

(fn ConstructionScript)

(fn GetCamera
  (return 0))

(fn GetItemData
  (return ""))