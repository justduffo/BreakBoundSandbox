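; Base interactable door actor that swings open and closed, with configurable meshes, starting state and swing side set in the construction script.
; Interaction plays or reverses a timeline that rotates the door, guarded against retriggering mid-swing.
; When locked, it searches the interaction component's keys for its KeyID, then either unlocks or plays a separate forced-open timeline.
; Open, close, unlock and force events play sounds at the door's cached location.
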(event Custom|DoorOpenSound
  ;[0.2275 0.2275 0.2275 0.502] Sound Handling
  ;;[0.2275 0.2275 0.2275 0.502] Open Door sound
  (Audio|PlaySoundatLocation (Variables|Sounds|GetOpenSound) (Variables|Default|GetDoorLocation) "0, 0, 0" 1.0 1.0 0.0 0 0 0 0))

(event Custom|DoorCloseSound
  ;[0.2275 0.2275 0.2275 0.502] Sound Handling
  ;;[0.2275 0.2275 0.2275 0.502] Close Door Sound
  (Utilities|FlowControl|Delay 0.5)
  (Audio|PlaySoundatLocation (Variables|Sounds|GetCloseSound) (Variables|Default|GetDoorLocation) "0, 0, 0" 1.0 1.0 0.0 0 0 0 0))

(event Custom|ForceToOpen
  ;[0.2275 0.2275 0.2275 0.502] Sound Handling
  ;;[0.2275 0.2275 0.2275 0.502] Force Open Sound
  (Audio|PlaySoundatLocation (Variables|Sounds|GetForceSound) (Variables|Default|GetDoorLocation) "0, 0, 0" 1.0 1.0 0.0 0 0 0 0))

(event Custom|UnlockDoor
  ;[0.2275 0.2275 0.2275 0.502] Sound Handling
  ;;[0.2275 0.2275 0.2275 0.502] Unlock Door Sound
  (Audio|PlaySoundatLocation (Variables|Sounds|GetUnlockSound) (Variables|Default|GetDoorLocation) "0, 0, 0" 1.0 1.0 0.0 0 0 0 0))

(event Custom|ForceOpenLockDoor
  ;[0.2275 0.2275 0.2275 0.502] Force to open locked door
  (CallFunction|ForcetoOpen)
  (bind _alpha (Timeline|TL_ForceOpen PlayFromStart)
    (:Update
      (Transformation|SetRelativeRotation (Variables|Default|GetDoor) (Math|Rotator|MakeRotator 0.0 0.0 _alpha) false false))))

(event EventBeginPlay
  ;[0.2275 0.2275 0.2275 0.502] Begin Play
  (Variables|Default|SetDoorLocation (Transformation|GetWorldLocation (Variables|Default|GetDoor))))

(event EventOnInteract
  ;[0.2275 0.2275 0.2275 0.502] Door Interaction
  (if (Variables|Settings|GetbIsLocked)
    (|KeyLogic
      (:True
        _)))
  (if (not (Audio|Components|Audio|IsPlaying (Variables|Default|GetTL_Doorstate)))
    (if (Variables|Settings|GetbIsClosed)
      (Variables|Settings|SetbIsClosed false)
      (CallFunction|DoorOpenSound)
      (bind _alpha (Timeline|TL_Doorstate PlayFromStart)
        (:Update
          (Transformation|SetRelativeRotation (Variables|Default|GetDoor) (Math|Rotator|MakeRotator 0.0 0.0 (Math|Float|Lerp 0.0 (Math|Float|SelectFloat 85.0 -85.0 (Variables|Settings|GetInvert)) _alpha)) false false)))
      (else
        (Variables|Settings|SetbIsClosed true)
        (CallFunction|DoorCloseSound)
        (Timeline|TL_Doorstate ReverseFromEnd)))))

(fn ConstructionScript
  (Components|StaticMesh|SetStaticMesh (Variables|Default|GetDoor) (Variables|Mesh|GetDoorMesh))
  (Components|StaticMesh|SetStaticMesh (Variables|Default|GetDoorFrame) (Variables|Mesh|GetDoorFrameMesh))
  (if (Variables|Settings|GetbIsClosed)
    (Transformation|SetRelativeRotation (Variables|Default|GetDoor) "0.0,0.0,0.0" false false)
    (elif (Variables|Settings|GetInvert)
      (Transformation|SetRelativeRotation (Variables|Default|GetDoor) "0.000000,-85.000000,0.000000" false false)
      (else
        (Transformation|SetRelativeRotation (Variables|Default|GetDoor) "0.000000,85.000000,0.000000" false false)))))

(fn SearchforKey
  (params (Keys :type Array%20of%20Integers))
  (bind _array_element (Utilities|Array|ForEachLoopwithBreak Keys :!label _label)
    (:LoopBody
      (if (== _array_element (Variables|Settings|GetKeyID))
        (Variables|Default|SetBIsKeyFound true)
        (goto _label Break)))
    (:Completed
      (return (Variables|Default|GetBIsKeyFound)))))

(fn GetCamera
  (return 0))

(fn GetItemData
  (return ""))